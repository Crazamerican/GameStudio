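; ScoreHolder persists the high score and last cleared level through a save slot and provides a vector randomization utility.
; LoadGame restores the high score but resets LastClearedLevel to zero, and calls SaveGame if no save exists.
; ShuffleVector keeps X and repeatedly applies ShuffleHelper's clamped random Y/Z offsets, compounding them until ShuffleCheck accepts the Y+Z sum range and minimum relative change from the original.
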(fn `LoadGame`
  (bind _savename (`self.SaveName`))
  (bind _returnvalue (`GameplayStatics.DoesSaveGameExist` _savename))
  (if _returnvalue
    (`KismetSystemLibrary.PrintString` "Loading Successful" true true (struct :`G` 0.66 :`B` 1.0 :`A` 1.0) 5.0)
    (bind _returnvalue_2 (`GameplayStatics.LoadGameFromSlot` _savename))
    (bind _assave_game (cast `/Game/Blueprints/SaveGame` _returnvalue_2))
    (set `self.Highscore` (`/Game/Blueprints/SaveGame.Highscore` _assave_game))
    (set `self.LastClearedLevel` 0)
    (else
      (`self.SaveGame`))))

(fn `SaveGame`
  (bind _returnvalue (`GameplayStatics.CreateSaveGameObject` "/Game/Blueprints/SaveGame.SaveGame_C"))
  (bind _output_get (set `self.Save Game Instance` _returnvalue))
  (set `/Game/Blueprints/SaveGame.Highscore` (`self.Highscore`) _output_get)
  (set `/Game/Blueprints/SaveGame.LastClearedLevel` (`self.LastClearedLevel`) _output_get)
  (`GameplayStatics.SaveGameToSlot` _output_get (`self.SaveName`))
  (`KismetSystemLibrary.PrintString` "Game Saved"))

(fn `ShuffleCheck`
  (params (CheckVector :type "Vector Structure") (OrigVector :type "Vector Structure") (Dif :type "Float (double-precision)"))
  (returns (Useable :type Boolean))
  (locals (DifZ :type "Float (double-precision)") (DifY :type "Float (double-precision)"))
  (bind _y (.y OrigVector))
  (bind _z (.z OrigVector))
  (bind _y_2 (.y CheckVector))
  (bind _z_2 (.z CheckVector))
  (bind _returnvalue (+ _y_2 _z_2))
  (set `local.DifY` (`KismetMathLibrary.Abs` (/ (- _y _y_2) _y)))
  (set `local.DifZ` (`KismetMathLibrary.Abs` (/ (- _z _z_2) _z)))
  (if (< _returnvalue 4.0)
    (if (> _returnvalue 2.0)
      (if (> (`local.DifY`) Dif)
        (if (>= (`local.DifZ`) Dif)
          (return true)
          (else
            _)))))
  (return false))

(fn `ShuffleHelper`
  (params (aVector :type "Vector Structure"))
  (returns (rVector :type "Vector Structure"))
  (locals (DifX :type "Float (double-precision)") (DifY :type "Float (double-precision)") (Size :type Boolean))
  (return (`KismetMathLibrary.MakeVector` (.x aVector) (`KismetMathLibrary.FClamp` (+ (.y aVector) (`KismetMathLibrary.RandomFloatInRange` -1.5 1.5)) 0.2 3.0) (`KismetMathLibrary.FClamp` (+ (.z aVector) (`KismetMathLibrary.RandomFloatInRange` -1.5 1.5)) 0.2 3.0))))

(fn `ShuffleVector`
  (params (Vec :type "Vector Structure") (MinDif :type "Float (double-precision)"))
  (returns (RetVec :type "Vector Structure"))
  (locals (DifY :type "Float (double-precision)" :default 0.0) (ChangeVector :type "Vector Structure") (Size :type Boolean :default true) (DifZ :type "Float (double-precision)"))
  (bind _output_get (set `local.ChangeVector` Vec))
  (bind _rvector (`self.ShuffleHelper` _output_get :!label _label))
  (bind _output_get_2 (set `local.ChangeVector` _rvector))
  (bind _useable (`self.ShuffleCheck` _output_get_2 Vec MinDif))
  (if _useable
    (return _output_get_2)
    (else
      (goto _label))))